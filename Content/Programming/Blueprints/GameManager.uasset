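; GameManager is an actor that runs the turn cycle of a game in which players roll and then shop.
; Left clicks step a TurnPhase state machine: roll the current Player, wait briefly in Rolling, then go from Choosing to opening the shop with the cursor shown.
; It creates the Menu widget on BeginPlay, and its shop-closed event calls AdvanceTurn to set the next Player and reset the phase.
; Right click during Choosing is an empty stub.
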(event `Key|LeftMouseButton`
  (params (Key :type "Key Structure"))
  (:`Pressed`
    (switch `/Game/Programming/Blueprints/PlayerState` (`self.TurnPhase`)
      (:`NewEnumerator0`
        (set `self.TurnPhase` "NewEnumerator1")
        (`PlayerPiece.Roll` (`self.player`))
        (`KismetSystemLibrary.Delay` 0.6)
        (set `self.TurnPhase` "NewEnumerator3"))
      (:`NewEnumerator3`
        (set `self.TurnPhase` "NewEnumerator2")
        (`/Game/UI/Menu.ShowShop` (`self.Menu Ref`) true)
        (set `PlayerController.bShowMouseCursor` true (`GameplayStatics.GetPlayerController` 0))))))

(event `self.ReceiveBeginPlay`
  (bind _returnvalue (`|CreateWidget` "/Game/UI/Menu.Menu_C" (`GameplayStatics.GetPlayerController` 0)))
  (set `self.Menu Ref` _returnvalue)
  (add `/Game/UI/Menu.OnShopClosed` (`self.Menu Ref`) (delegate `EndTurn`))
  (`UserWidget.AddToViewport` (`self.Menu Ref`) 0))

(event `EndTurn`
  (bind _returnvalue (`self.AdvanceTurn`))
  (set `self.player` _returnvalue)
  (set `self.TurnPhase` "NewEnumerator0"))

(event `Key|RightMouseButton`
  (params (Key :type "Key Structure"))
  (:`Pressed`
    (if (`|EnumEquality` (`self.TurnPhase`) "NewEnumerator3")
      _)))

(fn `UserConstructionScript`)